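; Player state Blueprint that tracks a player's score.
; AddScore adds to the running total and broadcasts the new value through the OnChangeScore event of an event subsystem.
; On BeginPlay it resets the score to zero and binds to that same event, printing each broadcast score with its own display name as a debug message.
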(event Custom|OnChangeScore_Event
  (params (Score :type Float%20%28double-precision%29))
  (Development|PrintString (Utilities|String|Append "NewScore" (Utilities|String|ToString(Float) Score) " - " "Source: " (Utilities|GetDisplayName self))))

(event EventBeginPlay
  (Variables|Default|SetScorePlayer 0.0)
  (EventDispatchers|AssignOnChangeScore (Subsystems|GetBPEventSubSystem) (delegate Custom|OnChangeScore_Event)))

(fn ConstructionScript)

(fn AddScore
  (params (NewScore :type Float%20%28double-precision%29))
  (bind _output_get (Variables|Default|SetScorePlayer (+ NewScore (Variables|Default|GetScorePlayer))))
  (Default|CallOnChangeScore (Subsystems|GetBPEventSubSystem) _output_get))