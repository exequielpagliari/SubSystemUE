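; BP_Cheat is a set of debug cheat functions for changing audio, graphics and radio settings.
; Audio functions set master, music and SFX volume, linearly or logarithmically, through the Sound subsystem.
; Graphics functions list available resolutions, apply one by index as fullscreen or windowed, and set global quality, saving via the Graphics subsystem.
; Radio functions skip to the next or previous track through the Radio subsystem.
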(fn AudioSetMusicVolumen
  (params (Volumen :type Float%20%28double-precision%29))
  (Class|SoundSubsystem|SetMusicVolume (Subsystems|GetSoundSubsystem) Volumen))

(fn GraphicsSetResolutionFullScreen
  (params (ValueGraph :type Integer))
  (bind _returnvalue (Subsystems|GetGraphicsSubsystem))
  (bind _returnvalue_2 (Class|GraphicsSubsystem|GetAvailableScreenResolutions _returnvalue))
  (Class|GraphicsSubsystem|SetResolution _returnvalue (.x (Utilities|Array|Get(acopy) _returnvalue_2 ValueGraph)) (.y (Utilities|Array|Get(acopy) _returnvalue_2 ValueGraph)) true)
  (Development|PrintString (Utilities|String|Append "X: " (Utilities|String|ToString(Integer) (.x (Utilities|Array|Get(acopy) _returnvalue_2 ValueGraph))) " Y: " (Utilities|String|ToString(Integer) (.y (Utilities|Array|Get(acopy) _returnvalue_2 ValueGraph)))))
  (Class|GraphicsSubsystem|ApplyandSaveSettings _returnvalue))

(fn GraphicsGetResolutions
  (bind _returnvalue (Class|GraphicsSubsystem|GetAvailableScreenResolutions (Subsystems|GetGraphicsSubsystem)))
  (for (_array_element _array_index) _returnvalue
    (Development|PrintString (Utilities|String|Append (Utilities|String|ToString(Integer) _array_index) "-  Resolution: " (Class|GraphicsSubsystem|ResolutiontoString (Subsystems|GetGraphicsSubsystem) _array_element)))))

(fn RadioPlayNextTrackRadio
  (Class|RadioSubsystem|PlayNextTrack (Subsystems|GetRadioSubsystem)))

(fn AudioSetMusicLogVolumen
  (params (Volumen :type Float%20%28double-precision%29))
  (Class|SoundSubsystem|SetMusicVolumeLogarithmic (Subsystems|GetSoundSubsystem) Volumen))

(fn GraphicsSetResolutionWindowed
  (params (ValueGraph :type Integer))
  (bind _returnvalue (Subsystems|GetGraphicsSubsystem))
  (bind _returnvalue_2 (Class|GraphicsSubsystem|GetAvailableScreenResolutions _returnvalue))
  (Class|GraphicsSubsystem|SetResolution _returnvalue (.x (Utilities|Array|Get(acopy) _returnvalue_2 ValueGraph)) (.y (Utilities|Array|Get(acopy) _returnvalue_2 ValueGraph)) false)
  (Development|PrintString (Utilities|String|Append "X: " (Utilities|String|ToString(Integer) (.x (Utilities|Array|Get(acopy) _returnvalue_2 ValueGraph))) " Y: " (Utilities|String|ToString(Integer) (.y (Utilities|Array|Get(acopy) _returnvalue_2 ValueGraph)))))
  (Class|GraphicsSubsystem|ApplyandSaveSettings _returnvalue))

(fn GraphicsSetQualityGlobal
  (params (QualityLevel :type Integer))
  (bind _returnvalue (Subsystems|GetGraphicsSubsystem))
  (Class|GraphicsSubsystem|SetScalabilityGroup _returnvalue QualityLevel)
  (Class|GraphicsSubsystem|ApplyandSaveSettings _returnvalue))

(fn AudioSetSFXVolumen
  (params (Volumen :type Float%20%28double-precision%29))
  (Class|SoundSubsystem|SetSFXVolume (Subsystems|GetSoundSubsystem) Volumen))

(fn AudioSetMasterVolumen
  (params (Volumen :type Float%20%28double-precision%29))
  (Class|SoundSubsystem|SetMasterVolume (Subsystems|GetSoundSubsystem) Volumen))

(fn RadioPlayPrevTrackRadio
  (Class|RadioSubsystem|PlayPreviousTrack (Subsystems|GetRadioSubsystem)))

(fn AudioSetSFXLogVolumen
  (params (Volumen :type Float%20%28double-precision%29))
  (Class|SoundSubsystem|SetSFXVolumeLogarithmic (Subsystems|GetSoundSubsystem) Volumen))

(fn AudioSetMasterLogVolumen
  (params (Volumen :type Float%20%28double-precision%29))
  (Class|SoundSubsystem|SetMasterVolumeLogarithmic (Subsystems|GetSoundSubsystem) Volumen))