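; AC_HealthComponent is an actor component that tracks its owner's health.
; On BeginPlay it fills health to max and binds to the owner's damage and hit events.
; Damage reduces health, clamped at zero, then broadcasts a damaged dispatcher, plus a dead dispatcher when health is zero.
; Actor hits only print the touched actor's name.
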(event Custom|OnActorHit_Event
  (params (SelfActor :type Actor%20Object%20Reference) (OtherActor :type Actor%20Object%20Reference) (NormalImpulse :type Vector) (Hit :type Hit%20Result%20Structure%20%28by%20ref%29))
  (Development|PrintString (Utilities|String|Append "TouchedActor: " (Utilities|GetDisplayName OtherActor))))

(event Custom|OnTakeAnyDamage_Event
  (params (DamagedActor :type Actor%20Object%20Reference) (Damage :type Float%20%28single-precision%29) (DamageType :type Damage%20Type%20Object%20Reference) (InstigatedBy :type Controller%20Object%20Reference) (DamageCauser :type Actor%20Object%20Reference))
  (CallFunction|DamageTaken DamagedActor Damage DamageType InstigatedBy DamageCauser))

(event EventBeginPlay
  (bind _returnvalue (Components|GetOwner))
  (Variables|Default|Set_currentHealth (Variables|Default|Get_maxHealth))
  (EventDispatchers|AssignOnTakeAnyDamage _returnvalue (delegate Custom|OnTakeAnyDamage_Event))
  (Collision|AssignOnActorHit _returnvalue (delegate Custom|OnActorHit_Event)))

(fn DamageTaken
  (params (damagedActor :type Actor%20Object%20Reference) (damage :type Float%20%28double-precision%29) (damageType :type Damage%20Type%20Object%20Reference) (instigator :type Controller%20Object%20Reference) (causer :type Actor%20Object%20Reference))
  (Variables|Default|Set_currentHealth (Math|Float|Max(Float) (- (Variables|Default|Get_currentHealth) damage) 0.0))
  (Default|CallOnComponentDamaged instigator damage (Variables|Default|Get_currentHealth))
  (if (<= (Variables|Default|Get_currentHealth) 0.0)
    (Default|CallOnComponentDead instigator)))